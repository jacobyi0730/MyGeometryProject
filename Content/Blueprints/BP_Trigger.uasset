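; BP_Trigger controls a pair of left and right doors that swing between open and closed rotations, starting closed at BeginPlay.
; DoOpen and DoClose set target rotations for both doors and a DoorOpen flag, which IsDoorOpen exposes.
; Tick eases each door toward its target with a fixed-alpha rotator lerp, so swing speed depends on frame rate.
; Despite the name, it has no active overlap logic of its own.
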(event EventBeginPlay
  (CallFunction|DoClose))

(event EventTick
  (params (DeltaSeconds :type Float%20%28single-precision%29))
  (bind _doorleft (Variables|Default|GetDoorLeft))
  (bind _doorright (Variables|Default|GetDoorRight))
  (Transformation|SetActorRotation _doorleft (Math|Rotator|Lerp(Rotator) (Transformation|GetActorRotation _doorleft) (Variables|Default|GetLeftDoorRot) 0.1))
  (Transformation|SetActorRotation _doorright (Math|Rotator|Lerp(Rotator) (Transformation|GetActorRotation _doorright) (Variables|Default|GetRightDoorRot) 0.1)))

(event Collision|EventActorBeginOverlap
  (params (OtherActor :type Actor%20Object%20Reference)))

(fn ConstructionScript)

(fn IsDoorOpen
  (return (Variables|Default|GetbDoorOpen)))

(fn DoOpen
  (Variables|Default|SetLeftDoorRot (Variables|Default|GetLeftOpen))
  (Variables|Default|SetRightDoorRot (Variables|Default|GetRightOpen))
  (Variables|Default|SetbDoorOpen true))

(fn DoClose
  (Variables|Default|SetLeftDoorRot (Variables|Default|GetLeftClose))
  (Variables|Default|SetRightDoorRot (Variables|Default|GetRightClose))
  (Variables|Default|SetbDoorOpen false))